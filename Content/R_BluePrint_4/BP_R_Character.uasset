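; Player character with walk/look controls that lets the user adjust the level's SunSky date and time.
; BeginPlay caches SunSky settings and creates main, fly-camera and superman-mode widgets, showing only the main one.
; Holding numpad +/- scrubs SolarTime on Tick and updates Hour/Minutes; U/I and O/P step day and month, clamped to non-leap month lengths.
; CameraFly spawns and possesses a BP_Spectator at the CineCamera, switching widgets.
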(event EventBeginPlay
  ;[1 1 1] Начальные значения
  (bind _returnvalue (Actor|GetActorOfClass "/SunPosition/SunSky.SunSky_C"))
  (Variables|Default|SetDay (Variables|/SunPosition/SunSky.SunSky_C|GetDay _returnvalue))
  (Variables|Default|SetMonth (Variables|/SunPosition/SunSky.SunSky_C|GetMonth _returnvalue))
  (Variables|Default|SetLantitude (Variables|/SunPosition/SunSky.SunSky_C|GetLatitude _returnvalue))
  (Variables|Default|SetLongitude (Variables|/SunPosition/SunSky.SunSky_C|GetLongitude _returnvalue))
  (Variables|Default|SetTimeZone (Variables|/SunPosition/SunSky.SunSky_C|GetTimeZone _returnvalue))
  (bind _output_get (Variables|Default|SetCarrent_SolarTime (Variables|/SunPosition/SunSky.SunSky_C|GetSolarTime _returnvalue)))
  (Variables|Default|SetHour (Math|Float|Truncate _output_get))
  (Variables|Default|SetMinutes (Math|Float|Truncate (/ (* 100 (Math|Float|%(Float) _output_get 1.0)) 1.66)))
  (bind _returnvalue_2 (UserInterface|CreateWidget "/Game/R_Widget/WBP_Main.WBP_Main_C"))
  (bind _output_get_2 (Variables|Default|SetMainWidget _returnvalue_2))
  (UserInterface|Viewport|AddtoViewport _output_get_2 0)
  (Widget|SetVisibility _output_get_2 "Visible")
  (bind _returnvalue_3 (UserInterface|CreateWidget "/Game/R_Widget/WBP_FlyCamera.WBP_FlyCamera_C"))
  (bind _output_get_3 (Variables|Default|SetFlyCam _returnvalue_3))
  (UserInterface|Viewport|AddtoViewport _output_get_3 0)
  (Widget|SetVisibility _output_get_3 "Hidden")
  (bind _returnvalue_4 (UserInterface|CreateWidget "/Game/R_Widget/WBP_SuopermanMode.WBP_SuopermanMode_C"))
  (bind _output_get_4 (Variables|Default|SetSuperMan _returnvalue_4))
  (UserInterface|Viewport|AddtoViewport _output_get_4 0)
  (Widget|SetVisibility _output_get_4 "Hidden"))

(event EventTick
  (params (DeltaSeconds :type Float%20%28single-precision%29))
  ;[1 1 1] Движение солнца
  (bind _returnvalue (Actor|GetActorOfClass "/SunPosition/SunSky.SunSky_C"))
  (if (Variables|Default|GetGroosMove)
    (if (Variables|Default|GetCheck_Press_Key)
      (if (< (+ (* DeltaSeconds (Variables|Default|GetSpeed_Sun_Move)) (Variables|/SunPosition/SunSky.SunSky_C|GetSolarTime _returnvalue)) 24.0)
        (Variables|/SunPosition/SunSky.SunSky_C|SetSolarTime _returnvalue (+ (* DeltaSeconds (Variables|Default|GetSpeed_Sun_Move)) (Variables|/SunPosition/SunSky.SunSky_C|GetSolarTime _returnvalue)))
        (Variables|Default|SetHour (Math|Float|Truncate (Variables|/SunPosition/SunSky.SunSky_C|GetSolarTime _returnvalue)))
        (Variables|Default|SetMinutes (Math|Float|Truncate (/ (* (Math|Float|%(Float) (Variables|/SunPosition/SunSky.SunSky_C|GetSolarTime _returnvalue) 1.0) 1e+02) 1.66)))))
    (elif (Variables|Default|GetDown_Move)
      (if (stale Input|KeyboardEvents|Subtract _output_get)
        (if (Variables|Default|GetCheck_Press_Key)
          (if (> (- (Variables|/SunPosition/SunSky.SunSky_C|GetSolarTime _returnvalue) (* DeltaSeconds (Variables|Default|GetSpeed_Sun_Move))) 0.0)
            (Variables|/SunPosition/SunSky.SunSky_C|SetSolarTime _returnvalue (- (Variables|/SunPosition/SunSky.SunSky_C|GetSolarTime _returnvalue) (* DeltaSeconds (Variables|Default|GetSpeed_Sun_Move))))
            (Variables|Default|SetHour (Math|Float|Truncate (Variables|/SunPosition/SunSky.SunSky_C|GetSolarTime _returnvalue)))
            (Variables|Default|SetMinutes (Math|Float|Truncate (/ (* (Math|Float|%(Float) (Variables|/SunPosition/SunSky.SunSky_C|GetSolarTime _returnvalue) 1.0) 1e+02) 1.66)))))))))

(event Collision|EventActorBeginOverlap
  (params (OtherActor :type Actor%20Object%20Reference)))

(event Input|ActionEvents|InputActionCameraFly
  (params (Key :type Key%20Structure :default "None"))
  (:Pressed
    (Widget|SetVisibility (Variables|Default|GetFlyCam) "Visible")
    (bind _returnvalue (Game|SpawnActorfromClass "/Game/R_BluePrint_4/BP_Spectator.BP_Spectator_C" (Transformation|GetWorldTransform (Variables|Default|GetCineCamera)) "AdjustIfPossibleButAlwaysSpawn" 0 0))
    (Pawn|Possess (Game|GetPlayerController 0) _returnvalue)
    (Widget|SetVisibility (Variables|Default|GetMainWidget) "Hidden")
    (Widget|SetVisibility (Variables|Default|GetSuperMan) "Hidden")
    (Pawn|Components|CharacterMovement|SetMovementMode (Variables|Character|GetCharacterMovement) "MOVE_Walking" 0)
    (Collision|SetCollisionEnabled (Variables|Collision|GetCapsuleComponent) "QueryAndPhysics")))

(event Input|AxisEvents|InputAxisMoveForward
  (params (AxisValue :type Float%20%28single-precision%29))
  ;[1 1 1] Движение персонажа в обычном режиме
  (Pawn|Input|AddMovementInput (Math|Vector|GetForwardVector (Variables|Collision|GetCapsuleComponent)) AxisValue false))

(event Input|AxisEvents|InputAxisMoveRight
  (params (AxisValue :type Float%20%28single-precision%29))
  ;[1 1 1] Движение персонажа в обычном режиме
  (Pawn|Input|AddMovementInput (Math|Vector|GetRightVector (Variables|Collision|GetCapsuleComponent)) AxisValue false))

(event Input|AxisEvents|InputAxisLookUp
  (params (AxisValue :type Float%20%28single-precision%29))
  ;[1 1 1] Движение персонажа в обычном режиме
  (Pawn|Input|AddControllerPitchInput AxisValue))

(event Input|AxisEvents|InputAxisTurn
  (params (AxisValue :type Float%20%28single-precision%29))
  ;[1 1 1] Движение персонажа в обычном режиме
  (Pawn|Input|AddControllerYawInput AxisValue))

(event Input|KeyboardEvents|U
  (params (Key :type Key%20Structure :default "None"))
  ;[1 1 1] Установка дня
  (:Pressed
    (switch int (Variables|Default|GetMonth)
      (:1
        (if (< (Variables|Default|GetDay) 31) :!label _label
          (bind _result (Math|Integer|IncrementInt (Variables|Default|GetDay))
            (:%20%20
              (Variables|/SunPosition/SunSky.SunSky_C|SetDay (stale EventTick _returnvalue) _result)))))
      (:2
        (if (< (Variables|Default|GetDay) 28)
          (bind _result_2 (Math|Integer|IncrementInt (Variables|Default|GetDay))
            (:%20%20
              (Variables|/SunPosition/SunSky.SunSky_C|SetDay (stale EventTick _returnvalue) _result_2)))))
      (:3
        (goto _label))
      (:4
        (if (< (Variables|Default|GetDay) 30) :!label _label_2
          (bind _result_3 (Math|Integer|IncrementInt (Variables|Default|GetDay))
            (:%20%20
              (Variables|/SunPosition/SunSky.SunSky_C|SetDay (stale EventTick _returnvalue) _result_3)))))
      (:5
        (goto _label))
      (:6
        (goto _label_2))
      (:7
        (goto _label))
      (:8
        (goto _label))
      (:9
        (goto _label_2))
      (:10
        (goto _label))
      (:11
        (goto _label_2))
      (:12
        (goto _label)))))

(event Input|KeyboardEvents|I
  (params (Key :type Key%20Structure :default "None"))
  ;[1 1 1] Установка дня
  (:Pressed
    (switch int (Variables|Default|GetMonth)
      (:1
        (if (> (Variables|Default|GetDay) 1) :!label _label
          (bind _result (Math|Integer|DecrementInt (Variables|Default|GetDay))
            (:%20%20
              (Variables|/SunPosition/SunSky.SunSky_C|SetDay (stale EventTick _returnvalue) _result)))))
      (:2
        (if (> (Variables|Default|GetDay) 1)
          (bind _result_2 (Math|Integer|DecrementInt (Variables|Default|GetDay))
            (:%20%20
              (Variables|/SunPosition/SunSky.SunSky_C|SetDay (stale EventTick _returnvalue) _result_2)))))
      (:3
        (goto _label))
      (:4
        (if (> (Variables|Default|GetDay) 1) :!label _label_2
          (bind _result_3 (Math|Integer|DecrementInt (Variables|Default|GetDay))
            (:%20%20
              (Variables|/SunPosition/SunSky.SunSky_C|SetDay (stale EventTick _returnvalue) _result_3)))))
      (:5
        (goto _label))
      (:6
        (goto _label_2))
      (:7
        (goto _label))
      (:8
        (goto _label))
      (:9
        (goto _label_2))
      (:10
        (goto _label))
      (:11
        (goto _label_2))
      (:12
        (goto _label)))))

(event Input|KeyboardEvents|Add
  (params (Key :type Key%20Structure :default "None"))
  ;[1 1 1] Движение солнца
  (:Pressed
    (Variables|Default|SetCheck_Press_Key true)
    (Variables|Default|SetGroosMove true))
  (:Released
    (Variables|Default|SetCheck_Press_Key false)
    (Variables|Default|SetGroosMove false)))

(event Input|KeyboardEvents|Subtract
  (params (Key :type Key%20Structure :default "None"))
  ;[1 1 1] Движение солнца
  (:Pressed
    (bind _output_get (Variables|Default|SetCheck_Press_Key true))
    (Variables|Default|SetDown_Move true))
  (:Released
    (Variables|Default|SetCheck_Press_Key false)
    (Variables|Default|SetDown_Move false)))

(event Input|KeyboardEvents|O
  (params (Key :type Key%20Structure :default "None"))
  ;[1 1 1] Установка месяца
  (:Pressed
    (if (< (Variables|/SunPosition/SunSky.SunSky_C|GetMonth (stale EventTick _returnvalue)) 12)
      (bind _result (Math|Integer|IncrementInt (Variables|Default|GetMonth))
        (:%20%20
          (bind _output_get (Variables|/SunPosition/SunSky.SunSky_C|SetMonth (stale EventTick _returnvalue) _result))
          (switch int _output_get
            (:2
              (if (> (Variables|/SunPosition/SunSky.SunSky_C|GetDay (stale EventTick _returnvalue)) 28)
                (bind _output_get_2 (Variables|/SunPosition/SunSky.SunSky_C|SetDay (stale EventTick _returnvalue) 28))
                (Variables|Default|SetDay _output_get_2)))
            (:4
              (if (> (Variables|/SunPosition/SunSky.SunSky_C|GetDay (stale EventTick _returnvalue)) 30) :!label _label
                (bind _output_get_3 (Variables|/SunPosition/SunSky.SunSky_C|SetDay (stale EventTick _returnvalue) 30))
                (Variables|Default|SetDay _output_get_3)))
            (:6
              (goto _label))
            (:9
              (goto _label))
            (:11
              (goto _label))))))))

(event Input|KeyboardEvents|P
  (params (Key :type Key%20Structure :default "None"))
  ;[1 1 1] Установка месяца
  (:Pressed
    (if (> (Variables|/SunPosition/SunSky.SunSky_C|GetMonth (stale EventTick _returnvalue)) 1)
      (bind _result (Math|Integer|DecrementInt (Variables|Default|GetMonth))
        (:%20%20
          (bind _output_get (Variables|/SunPosition/SunSky.SunSky_C|SetMonth (stale EventTick _returnvalue) _result))
          (switch int _output_get
            (:2
              (if (> (Variables|/SunPosition/SunSky.SunSky_C|GetDay (stale EventTick _returnvalue)) 28)
                (bind _output_get_2 (Variables|/SunPosition/SunSky.SunSky_C|SetDay (stale EventTick _returnvalue) 28))
                (Variables|Default|SetDay _output_get_2)))
            (:4
              (if (> (Variables|/SunPosition/SunSky.SunSky_C|GetDay (stale EventTick _returnvalue)) 30) :!label _label
                (bind _output_get_3 (Variables|/SunPosition/SunSky.SunSky_C|SetDay (stale EventTick _returnvalue) 30))
                (Variables|Default|SetDay _output_get_3)))
            (:6
              (goto _label))
            (:9
              (goto _label))
            (:11
              (goto _label))))))))

(fn ConstructionScript)